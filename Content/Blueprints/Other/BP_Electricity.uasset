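; BP_Electricity is a power switch actor that turns electricity on or off for BP_AttribDoor doors.
; On BeginPlay, it gathers every BP_AttribDoor in the level if its Doors array is empty.
; Each overlap by the FirstPersonCharacter toggles IsOn, swaps the Cube material between green and red, and copies the state to each door's HaveElectricity flag.
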(event `self.ReceiveBeginPlay`
  (if (== (`KismetArrayLibrary.Array_Length` (`self.Doors`)) 0)
    (bind _outactors (`GameplayStatics.GetAllActorsOfClass` "/Game/Blueprints/Doors/BP_AttribDoor.BP_AttribDoor_C"))
    (set `self.Doors` _outactors)))

(event `self.ReceiveActorBeginOverlap`
  (params (OtherActor :type "Actor Object Reference"))
  (bind _cube (`self.Cube`))
  (cast `/Game/FirstPersonBP/Blueprints/FirstPersonCharacter` OtherActor)
  (bind _output_get (set `self.IsOn` (not (`self.IsOn`))))
  (if _output_get
    (`PrimitiveComponent.SetMaterial` _cube 0 "/Game/Materials/MI_Green.MI_Green")
    (else
      (`PrimitiveComponent.SetMaterial` _cube 0 "/Game/Materials/MI_Red.MI_Red")))
  (for _array_element (`self.Doors`)
    (set `/Game/Blueprints/Doors/BP_AttribDoor.HaveElectricity` (`self.IsOn`) _array_element)))

(fn `UserConstructionScript`)