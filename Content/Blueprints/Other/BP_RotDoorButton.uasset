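; BP_RotDoorButton is a button actor that controls a linked door, apparently a rotating one.
; Its PushButton event runs a FlipFlop that alternates between calling Move and Stop on the referenced Door.
; The BeginPlay, overlap and Tick events are disabled, so all behavior depends on PushButton being called from outside.
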(event `self.PushButton`
  (bind _door (`self.Door`))
  (`/Engine/EditorBlueprintResources/StandardMacros.FlipFlop`
    (:`A`
      (`/Game/Blueprints/Doors/BP_RotDoor.Move` _door))
    (:`B`
      (`/Game/Blueprints/Doors/BP_RotDoor.Stop` _door))))

(fn `UserConstructionScript`
  (`parent.UserConstructionScript`))