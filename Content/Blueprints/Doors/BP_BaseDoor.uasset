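; Base door actor that provides a hinged mesh setup and a common Open/Close interface.
; The construction script offsets DoorMesh to a front, middle or back pivot alignment, then yaws the Pivot component by Aperture or zero to match DoorState.
; Open and Close are empty stubs, GetAperture returns the opening angle, and the event graph holds no runtime logic.
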(fn `Close`)

(fn `GetAperture`
  (returns (Aperture :type "Float (double-precision)"))
  (return (`self.Aperture`)))

(fn `Open`)

(fn `UserConstructionScript`
  (bind _doormesh (`self.DoorMesh`))
  (bind _pivot (`self.Pivot`))
  (switch `/Game/Blueprints/Doors/E_DoorPivot` (`self.DoorPivot`)
    (:`NewEnumerator0`
      (`SceneComponent.K2_SetRelativeLocation` _doormesh (65.0 5.0 125.0) false false))
    (:`NewEnumerator1`
      (`SceneComponent.K2_SetRelativeLocation` _doormesh (65.0 0.0 125.0) false false))
    (:`NewEnumerator2`
      (`SceneComponent.K2_SetRelativeLocation` _doormesh (65.0 -5.0 125.0) false false)))
  (switch `/Game/Blueprints/Doors/E_DoorTwoStates` (`self.DoorState`)
    (:`NewEnumerator0`
      (`SceneComponent.K2_SetRelativeRotation` _pivot (`KismetMathLibrary.MakeRotator` 0.0 0.0 (`self.Aperture`)) false false))
    (:`NewEnumerator1`
      (`SceneComponent.K2_SetRelativeRotation` :`self` _pivot))))