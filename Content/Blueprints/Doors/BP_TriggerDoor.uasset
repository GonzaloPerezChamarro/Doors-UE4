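; BP_TriggerDoor is a door that opens when the FirstPersonCharacter overlaps the actor and closes when the overlap ends.
; Open plays a timeline and Close reverses it, with ApertureType choosing whether the vector output rotates the Pivot (Radial) or sets its relative location (Linear).
; BeginPlay injects the Curve asset into the timeline and matches its length to the curve's last key.
; The Linear branch also prints the curve value on each update.
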(event `self.ReceiveActorBeginOverlap`
  (params (OtherActor :type "Actor Object Reference"))
  (cast `/Game/FirstPersonBP/Blueprints/FirstPersonCharacter` OtherActor)
  (`self.Open`))

(event `self.ReceiveActorEndOverlap`
  (params (OtherActor :type "Actor Object Reference"))
  (cast `/Game/FirstPersonBP/Blueprints/FirstPersonCharacter` OtherActor)
  (`self.Close`))

(event `self.Open`
  (bind _pivot (`self.Pivot`))
  (bind (_direction _dooraperturecurve01) (`Timeline|DoorApertureTimeLine` :!label _label)
    (:`Update`
      (switch `/Game/Blueprints/Doors/E_ApertureType` (`self.ApertureType`)
        (:`NewEnumerator0`
          (`SceneComponent.K2_SetRelativeRotation` _pivot (`KismetMathLibrary.Conv_VectorToRotator` _dooraperturecurve01) false false))
        (:`NewEnumerator1`
          (`KismetSystemLibrary.PrintString` (`KismetStringLibrary.Conv_VectorToString` _dooraperturecurve01))
          (`SceneComponent.K2_SetRelativeLocation` _pivot _dooraperturecurve01 false false))))))

(event `self.Close`
  (goto _label :!via `Reverse`))

(event `self.ReceiveBeginPlay`
  (bind _dooraperturetimeline (`self.DoorApertureTimeLine`))
  (bind _curve (`self.Curve`))
  (`TimelineComponent.SetVectorCurve` _dooraperturetimeline _curve "DoorApertureCurve01")
  (`TimelineComponent.SetTimelineLength` _dooraperturetimeline (`.MaxTime` (`CurveBase.GetTimeRange` _curve))))

(fn `UserConstructionScript`
  (`parent.UserConstructionScript`))