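; Rotating door that spins its Pivot on Move and eases to a halt on Stop, guarded by an IsMoving flag.
; A SpeedChange timeline ramps the yaw increments up, hands over to TimeLine for continued rotation, and plays in reverse to wind down.
; Each Tick, if DoorMesh's physics yaw velocity exceeds 70 deg/s either way, it is reset to positive 70.
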(event `self.ReceiveTick`
  (params (DeltaSeconds :type "Float (single-precision)"))
  (bind (_returnvalue_x _returnvalue_y _returnvalue_z) (`KismetMathLibrary.BreakVector` (`PrimitiveComponent.GetPhysicsAngularVelocityInDegrees` (`self.DoorMesh`) "None")))
  (if (> (`KismetMathLibrary.Abs` _returnvalue_z) 70.0)
    (`PrimitiveComponent.SetAllPhysicsAngularVelocityInDegrees` (`self.DoorMesh`) (0.0 0.0 70.0) false)))

(event `Move`
  (if (not (`self.IsMoving`))
    (set `self.IsMoving` true)
    (bind (_direction _speed) (`Timeline|SpeedChange` :!via `PlayFromStart` :!label _label)
      (:`Update`
        (`SceneComponent.K2_AddRelativeRotation` (`self.Pivot`) (`KismetMathLibrary.MakeRotator` 0.0 0.0 (* _speed (`self.Speed`) 0.01)) false false))
      (:`Finished`
        (if (`self.IsMoving`)
          (bind (_direction_2 _tick) (`Timeline|TimeLine` :!via `PlayFromStart` :!label _label_2)
            (:`Update`
              (`SceneComponent.K2_AddRelativeRotation` (`self.Pivot`) (`KismetMathLibrary.MakeRotator` 0.0 0.0 (* _tick 0.01 (`self.Speed`))) false false))))))))

(event `Stop`
  (if (`self.IsMoving`)
    (`|ExecutionSequence`
      (:`then_0`
        (set `self.IsMoving` false)
        (goto _label_2 :!via `Stop`))
      (:`then_1`
        (goto _label :!via `ReverseFromEnd`)))))

(fn `UserConstructionScript`)