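; Interactable hinged door that swings open and closed, with blocked, electricity and key checks that print a message on refusal.
; Interact passes those checks, then Tick eases Pivot yaw toward the target until a timer ends the interaction, with StopInteract flipping the door state.
; Doors open left, right or, for Both, by dotting player mesh forward with CentralPoint's right vector.
; The construction script pre-rotates doors set to start open.
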(event `self.ReceiveTick`
  (params (DeltaSeconds :type "Float (single-precision)"))
  (`parent.ReceiveTick` DeltaSeconds)
  (if (`self.IsInteracting`)
    (`self.ManageDoor`)))

(event `/Game/Blueprints/BPI_Interactable.Interact`
  ;[1 1 1] Interaction
  (if (not (`self.IsInteracting`))
    (if (`self.IsBlocked`)
      (`/Engine/EditorBlueprintResources/StandardMacros.DoOnce` false :!label _label
        (:`Completed`
          (`KismetSystemLibrary.PrintString` "The door is blocked" true true (struct :`R` 0.515625 :`G` 0.129972 :`A` 1.0))
          (`KismetSystemLibrary.Delay` 1.0)
          (goto _label :!via `Reset`)))
      (elif (`self.NeedElectricity`)
        (if (`self.HaveElectricity`)
          (if (`self.NeedKey`) :!label _label_2
            (`KismetSystemLibrary.PrintString` "The door need a key" true true (struct :`R` 1.0 :`G` 0.787897 :`B` 0.123451 :`A` 1.0))
            (else
              (`self.Interaction`)))
          (else
            (`KismetSystemLibrary.PrintString` "The door need electricity" true true (struct :`R` 1.0 :`G` 0.948633 :`B` 0.568745 :`A` 1.0))))
        (else
          (goto _label_2))))))

(event `self.Open`
  ;[1 1 1] Open/Close
  (switch `/Game/Blueprints/Doors/E_ApertureType` (`self.ApertureType`)
    (:`NewEnumerator2`
      (bind _aperture (`self.GetAperture` :!label _label_3))
      (`self.RotateDoor` (* -1 _aperture)))
    (:`NewEnumerator3`
      (bind _aperture_2 (`self.GetAperture` :!label _label_4))
      (`self.RotateDoor` _aperture_2))
    (:`NewEnumerator4`
      (if (< (`KismetMathLibrary.Dot_VectorVector` (`SceneComponent.GetForwardVector` (`Character.Mesh` (`GameplayStatics.GetPlayerCharacter` 0))) (`SceneComponent.GetRightVector` (`self.CentralPoint`))) 0.0)
        (goto _label_3)
        (else
          (goto _label_4))))))

(event `self.Close`
  ;[1 1 1] Open/Close
  (`self.RotateDoor` 0.0))

(fn `Interaction`
  (set `self.IsInteracting` true)
  (`KismetSystemLibrary.K2_SetTimerDelegate` (`|CreateDelegate` :!event `StopInteract`) (`self.InteractionTime`)))

(fn `ManageDoor`
  (switch `/Game/Blueprints/Doors/E_DoorTwoStates` (`self.DoorState`)
    (:`NewEnumerator0`
      (`self.Close`))
    (:`NewEnumerator1`
      (`self.Open`))))

(fn `RotateDoor`
  (params (Rotation :type "Float (double-precision)"))
  (`SceneComponent.K2_SetRelativeRotation` (`self.pivot`) (`KismetMathLibrary.MakeRotator` 0.0 0.0 (`KismetMathLibrary.FInterpTo` (.yaw (`SceneComponent.RelativeRotation` (`self.pivot`))) Rotation (`GameplayStatics.GetWorldDeltaSeconds`) 3.0)) false false))

(fn `StopInteract`
  (set `self.IsInteracting` false)
  (switch `/Game/Blueprints/Doors/E_DoorTwoStates` (`self.DoorState`)
    (:`NewEnumerator0`
      (set `self.DoorState` "NewEnumerator1"))
    (:`NewEnumerator1`
      (set `self.DoorState` "NewEnumerator0"))))

(fn `UserConstructionScript`
  (bind _pivot (`self.Pivot`))
  (`parent.UserConstructionScript`)
  (switch `/Game/Blueprints/Doors/E_DoorTwoStates` (`self.DoorState`)
    (:`NewEnumerator0`
      (bind _aperture (`self.GetAperture`))
      (switch `/Game/Blueprints/Doors/E_ApertureType` (`self.ApertureType`)
        (:`NewEnumerator2`
          (`SceneComponent.K2_SetRelativeRotation` _pivot (`KismetMathLibrary.MakeRotator` 0.0 0.0 (* -1 _aperture)) false false :!label _label))
        (:`NewEnumerator3`
          (`SceneComponent.K2_SetRelativeRotation` _pivot (`KismetMathLibrary.MakeRotator` 0.0 0.0 _aperture) false false))
        (:`NewEnumerator4`
          (goto _label))))))