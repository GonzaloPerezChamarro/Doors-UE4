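; BP_SpringDoor is an interactable door that swings open, then slowly closes itself.
; Interact starts the opening; both branches of its facing check set the same swing direction.
; Tick eases the Pivot's yaw with FInterpTo toward the Aperture angle, snapping when nearly there.
; After a TimeToClose delay, it eases back at a slower speed whenever the first-person character is not overlapping the actor.
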(event `self.ReceiveTick`
  (params (DeltaSeconds :type "Float (single-precision)"))
  ;[1 1 1] Event Tick
  (if (`self.ShouldOpen`)
    (bind _rotation (`self.Open`))
    (bind _finished (`self.ManageOpening` _rotation))
    (if _finished
      (set `self.ShouldOpen` false)
      (`KismetSystemLibrary.Delay` (`self.TimeToClose`))
      (set `self.ShouldClose` true)
      (set `self.IsOpen` true))
    (elif (`self.IsOpen`)
      (if (not (`self.IsOverlapingRight`))
        (`self.Close`)
        (bind _finished_2 (`self.ManageOpening` 0.0))
        (if _finished_2
          (set `self.IsOpen` false))))))

(event `/Game/Blueprints/BPI_Interactable.Interact`
  ;[1 1 1] Interact
  (if (>= (`KismetMathLibrary.Dot_VectorVector` (`SceneComponent.GetForwardVector` (`Character.Mesh` (`GameplayStatics.GetPlayerCharacter` 0))) (`SceneComponent.GetForwardVector` (`self.Point`))) 0.0)
    (set `self.SideToOpen` -1)
    (else
      (set `self.SideToOpen` -1)))
  (set `self.ShouldOpen` true))

(event `self.ReceiveActorBeginOverlap`
  (params (OtherActor :type "Actor Object Reference"))
  ;[1 1 1] Overlaping
  (cast `/Game/FirstPersonBP/Blueprints/FirstPersonCharacter` OtherActor)
  (set `self.IsOverlapingRight` true))

(event `self.ReceiveActorEndOverlap`
  (params (OtherActor :type "Actor Object Reference"))
  ;[1 1 1] Overlaping
  (cast `/Game/FirstPersonBP/Blueprints/FirstPersonCharacter` OtherActor)
  (set `self.IsOverlapingRight` false))

(fn `Close`
  (`self.RotateDoor` 0.0 0.2))

(fn `ManageOpening`
  (params (Rotation :type "Float (double-precision)"))
  (returns (Finished :type Boolean))
  (bind _pivot (`self.Pivot`))
  (bind _returnvalue (`KismetMathLibrary.NearlyEqual_FloatFloat` (.yaw (`SceneComponent.RelativeRotation` _pivot)) Rotation 0.1))
  (if _returnvalue
    (`SceneComponent.K2_SetRelativeRotation` _pivot (`KismetMathLibrary.MakeRotator` 0.0 0.0 Rotation) false false))
  (return _returnvalue))

(fn `Open`
  (returns (Rotation :type "Float (double-precision)"))
  (bind _returnvalue (* (`self.SideToOpen`) (`self.Aperture`)))
  (`self.RotateDoor` _returnvalue 2.0)
  (return _returnvalue))

(fn `RotateDoor`
  (params (Rotation :type "Float (double-precision)") (`Interp Speed` :type "Float (double-precision)"))
  (`SceneComponent.K2_SetRelativeRotation` (`self.Pivot`) (`KismetMathLibrary.MakeRotator` 0.0 0.0 (`KismetMathLibrary.FInterpTo` (.yaw (`SceneComponent.RelativeRotation` (`self.Pivot`))) Rotation (`GameplayStatics.GetWorldDeltaSeconds`) `Interp Speed`)) false false))

(fn `UserConstructionScript`)