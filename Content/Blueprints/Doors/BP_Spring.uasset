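; Spring door that opens when interacted with and swings shut on its own after a delay.
; Tick eases the Pivot's yaw toward GetAperture, snaps it when nearly equal, then waits TimeToClose before switching DoorState to allow closing.
; Closing is slower than opening and advances only while the FirstPersonCharacter is not overlapping the actor.
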(event `self.ReceiveActorBeginOverlap`
  (params (OtherActor :type "Actor Object Reference"))
  ;[1 1 1] Overlaping
  (cast `/Game/FirstPersonBP/Blueprints/FirstPersonCharacter` OtherActor)
  (set `self.IsOverlaping` true))

(event `self.ReceiveActorEndOverlap`
  (params (OtherActor :type "Actor Object Reference"))
  ;[1 1 1] Overlaping
  (cast `/Game/FirstPersonBP/Blueprints/FirstPersonCharacter` OtherActor)
  (set `self.IsOverlaping` false))

(event `/Game/Blueprints/BPI_Interactable.Interact`
  ;[1 1 1] Interaction
  (if (not (`self.ShouldOpen`))
    (set `self.ShouldOpen` true)))

(event `self.ReceiveTick`
  (params (DeltaSeconds :type "Float (single-precision)"))
  ;[1 1 1] Event TIck
  (if (`self.ShouldOpen`)
    (`self.Open`)
    (bind _aperture (`self.GetAperture`))
    (bind _ended (`self.ManageOpening` _aperture))
    (if _ended
      (set `self.ShouldOpen` false)
      (`KismetSystemLibrary.Delay` (`self.TimeToClose`))
      (set `self.ShouldClose` true)
      (set `self.DoorState` "NewEnumerator0"))
    (elif (`|EnumEquality` (`self.DoorState`) "NewEnumerator0")
      (if (not (`self.IsOverlaping`))
        (`self.Close`)
        (bind _ended_2 (`self.ManageOpening` 0.0))
        (if _ended_2
          (set `self.DoorState` "NewEnumerator1"))))))

(event `self.Open`
  ;[1 1 1] Open/Close
  (bind _aperture (`self.GetAperture`))
  (`self.RotateDoor` _aperture 2.0))

(event `self.Close`
  ;[1 1 1] Open/Close
  (`self.RotateDoor` 0.0 0.4))

(fn `ManageOpening`
  (params (Rotation :type "Float (double-precision)"))
  (returns (Ended :type Boolean))
  (bind _pivot (`self.Pivot`))
  (bind _returnvalue (`KismetMathLibrary.NearlyEqual_FloatFloat` (.yaw (`SceneComponent.RelativeRotation` _pivot)) Rotation 0.1))
  (if _returnvalue
    (`SceneComponent.K2_SetRelativeRotation` _pivot (`KismetMathLibrary.MakeRotator` 0.0 0.0 Rotation) false false))
  (return _returnvalue))

(fn `RotateDoor`
  (params (Rotation :type "Float (double-precision)") (InterpSpeed :type "Float (double-precision)"))
  (`SceneComponent.K2_SetRelativeRotation` (`self.Pivot`) (`KismetMathLibrary.RInterpTo` (`SceneComponent.RelativeRotation` (`self.Pivot`)) (`KismetMathLibrary.MakeRotator` 0.0 0.0 Rotation) (`GameplayStatics.GetWorldDeltaSeconds`) InterpSpeed) false false))

(fn `UserConstructionScript`
  (`parent.UserConstructionScript`))