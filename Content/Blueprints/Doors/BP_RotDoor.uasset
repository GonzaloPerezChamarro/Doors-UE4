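; Rotating door actor that turns its Pivot around yaw on Move and winds down on Stop.
; The SpeedChange timeline ramps rotation up, then hands off to TimeLine; Stop plays SpeedChange in reverse, with IsMoving blocking the handoff.
; While moving, an overlap zeroes CurrentSpeed and its end restores Speed; that Move call is a no-op because IsMoving is still true.
; Rotation steps are per timeline update, without delta-time scaling.
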(event `self.ReceiveBeginPlay`
  (set `self.CurrentSpeed` (`self.Speed`)))

(event `Move`
  (if (not (`self.IsMoving`))
    (set `self.IsMoving` true)
    (bind (_direction _speed) (`Timeline|SpeedChange` :!via `PlayFromStart` :!label _label)
      (:`Update`
        (`SceneComponent.K2_AddRelativeRotation` (`self.Pivot`) (`KismetMathLibrary.MakeRotator` 0.0 0.0 (* _speed (`self.CurrentSpeed`) 0.01)) false false))
      (:`Finished`
        (if (`self.IsMoving`)
          (bind (_direction_2 _tick) (`Timeline|TimeLine` :!via `PlayFromStart` :!label _label_2)
            (:`Update`
              (`SceneComponent.K2_AddRelativeRotation` (`self.Pivot`) (`KismetMathLibrary.MakeRotator` 0.0 0.0 (* _tick 0.01 (`self.CurrentSpeed`))) false false))))))))

(event `Stop`
  (if (`self.IsMoving`)
    (`|ExecutionSequence`
      (:`then_0`
        (set `self.IsMoving` false)
        (goto _label_2 :!via `Stop`))
      (:`then_1`
        (goto _label :!via `ReverseFromEnd`)))))

(event `self.ReceiveActorBeginOverlap`
  (params (OtherActor :type "Actor Object Reference"))
  (if (`self.IsMoving`)
    (set `self.CurrentSpeed` 0.0)))

(event `self.ReceiveActorEndOverlap`
  (params (OtherActor :type "Actor Object Reference"))
  (if (`self.IsMoving`)
    (set `self.CurrentSpeed` (`self.Speed`))
    (`self.Move`)))

(fn `UserConstructionScript`)