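; BP_BasicDoor is an interactable swinging door that can be blocked, need electricity or need a key.
; Interact checks those conditions, printing the reason on failure, and otherwise flags the door as interacting and starts a timer.
; While flagged, Tick interpolates the Pivot yaw toward the open aperture or zero, based on DoorState.
; StopInteract clears the flag and flips DoorState; power status comes from a BP_Electricity actor, looked up if unset.
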(event `self.ReceiveBeginPlay`
  ;[1 1 1] Begin Play
  (if (== (`self.Electricity`) null)
    (bind _outactors (`GameplayStatics.GetAllActorsOfClass` "/Game/Blueprints/Other/BP_Electricity.BP_Electricity_C"))
    (set `self.Electricity` (`|GetArrayItem` _outactors))))

(event `self.ReceiveTick`
  (params (DeltaSeconds :type "Float (single-precision)"))
  ;[1 1 1] Event Tick
  (if (`self.IsInteracting`)
    (`self.ManageDoor`)))

(event `/Game/Blueprints/BPI_Interactable.Interact`
  ;[1 1 1] Interaction
  (if (not (`self.IsInteracting`))
    (if (`self.IsBlocked`)
      (`/Engine/EditorBlueprintResources/StandardMacros.DoOnce` false :!label _label
        (:`Completed`
          (`KismetSystemLibrary.PrintString` "The door is blocked" true true (struct :`R` 0.515625 :`G` 0.129972 :`A` 1.0))
          (`KismetSystemLibrary.Delay` 1.0)
          (goto _label :!via `Reset`)))
      (elif (`self.NeedElectricity`)
        (if (`/Game/Blueprints/Other/BP_Electricity.IsOn` (`self.Electricity`))
          (if (`self.NeedKey`) :!label _label_2
            (if (`self.HasKey`)
              (`self.Interaction` :!label _label_3)
              (else
                (`KismetSystemLibrary.PrintString` "The door need a key" true true (struct :`R` 1.0 :`G` 0.787897 :`B` 0.123451 :`A` 1.0))))
            (else
              (goto _label_3)))
          (else
            (`KismetSystemLibrary.PrintString` "The door need electricity" true true (struct :`R` 1.0 :`G` 0.948633 :`B` 0.568745 :`A` 1.0))))
        (else
          (goto _label_2))))))

(fn `Close`
  (`self.RotateDoor` 0.0))

(fn `Interaction`
  (set `self.IsInteracting` true)
  (`KismetSystemLibrary.K2_SetTimerDelegate` (`|CreateDelegate` :!event `StopInteract`) (`self.InteractionTime`)))

(fn `ManageDoor`
  (switch `/Game/Blueprints/Doors/E_DoorTwoStates` (`self.DoorState`)
    (:`NewEnumerator0`
      (`self.Close`))
    (:`NewEnumerator1`
      (`self.Open`))))

(fn `Open`
  (`self.RotateDoor` (`self.Aperture`)))

(fn `RotateDoor`
  (params (Rotation :type "Float (double-precision)"))
  (`SceneComponent.K2_SetRelativeRotation` (`self.pivot`) (`KismetMathLibrary.MakeRotator` 0.0 0.0 (`KismetMathLibrary.FInterpTo` (.yaw (`SceneComponent.RelativeRotation` (`self.pivot`))) Rotation (`GameplayStatics.GetWorldDeltaSeconds`) 3.0)) false false))

(fn `StopInteract`
  (set `self.IsInteracting` false)
  (switch `/Game/Blueprints/Doors/E_DoorTwoStates` (`self.DoorState`)
    (:`NewEnumerator0`
      (set `self.DoorState` "NewEnumerator1"))
    (:`NewEnumerator1`
      (set `self.DoorState` "NewEnumerator0"))))

(fn `UserConstructionScript`)